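; Game mode for Magus that spawns a wave of AI enemies as soon as play begins.
; BeginPlay runs StartGame, which calls SpawnEnemies to size the wave from CurrentWave and set the EnemiesLeft counter.
; Two loops split the EnemyAI spawns evenly between two spawn locations, the first breaking at the halfway index.
; Nothing in this graph advances the wave or decrements the counter.
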(event `self.ReceiveBeginPlay`
  (`self.Start Game`))

(event `Start Game`
  (`self.Spawn Enemies`))

(event `Spawn Enemies`
  (bind _output_get (set `self.EnemyTotal` (* (`self.CurrentWave`) 4)))
  (set `self.EnemiesLeft` _output_get)
  (for _index (range (+ _output_get 1))
    (if (== _index (/ (`self.EnemyTotal`) 2))
      (break)
      (else
        (`|SpawnActorFromClass` "/Game/Blueprints/Enemies/EnemyAI.EnemyAI_C" (`self.SpawnLocation1`) "Undefined" "MultiplyWithRoot" null null))))
  (for _ (range 1 (+ (/ (`self.EnemyTotal`) 2) 1))
    (`|SpawnActorFromClass` "/Game/Blueprints/Enemies/EnemyAI.EnemyAI_C" (`self.SpawnLocation2`) "Undefined" "MultiplyWithRoot" null null)))

(fn `UserConstructionScript`)