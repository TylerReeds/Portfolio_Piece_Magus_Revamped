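; Enemy AI Blueprint that chases the first player pawn once PawnSensing spots one.
; AIMoveTo success plays an attack montage, then calls ApplyDamage with no damaged actor wired, gated by a self "Player" tag check.
; The CanAttack cooldown and sphere-overlap hit check are disconnected.
; The damage handler's inverted Health check destroys the enemy while Health is positive, and Tick halts movement until a player is seen.
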(event `self.ReceiveAnyDamage`
  (params (Damage :type "Float (single-precision)") (DamageType :type "DamageType Object Reference") (InstigatedBy :type "Controller Object Reference") (DamageCauser :type "Actor Object Reference"))
  (if (<= (`self.health`) 0.0)
    (set `self.health` (- (`self.health`) Damage))
    (else
      (`self.K2_DestroyActor`))))

(event `self.ReceiveTick`
  (params (DeltaSeconds :type "Float (single-precision)"))
  (if (not (`self.isSeeingPlayer`))
    (`MovementComponent.StopMovementImmediately` (`self.CharacterMovement`))))

(event `self.PawnSensing.OnSeePawn`
  (params (Pawn :type "Pawn Object Reference"))
  (set `self.isSeeingPlayer` true)
  (`self.FollowPlayer`))

(event `FollowPlayer`
  (set `self.canAttack` true)
  (if (`self.isSeeingPlayer`)
    (`|AIMoveTo` self (0.0 0.0 0.0) (`GameplayStatics.GetPlayerPawn` 0)
      (:`OnSuccess`
        (if (`self.canAttack`)
          (set `self.canAttack` false)
          (bind _returnvalue (`self.PlayAnimMontage` null))
          (if (`self.ActorHasTag` "Player")
            (`GameplayStatics.ApplyDamage` null 25.0)))))
    (else
      (set `self.isSeeingPlayer` false))))

(fn `UserConstructionScript`)