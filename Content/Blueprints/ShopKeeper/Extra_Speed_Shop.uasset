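; Shop keeper Blueprint for the Extra Speed shop, which shows a prompt widget while something overlaps its Box collider.
; Begin and end overlap events toggle the visibility of that widget without filtering the overlapping actor.
; A ShopKeeperMenu event creates the Extra_Speed menu widget, adds it to the viewport, shows the mouse cursor, switches to UI-only input and pauses the game.
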(event `self.Box.OnComponentBeginOverlap`
  (params (OverlappedComponent :type "PrimitiveComponent Object Reference") (OtherActor :type "Actor Object Reference") (OtherComp :type "PrimitiveComponent Object Reference") (OtherBodyIndex :type Integer) (bFromSweep :type Boolean) (SweepResult :type "HitResult Structure (by ref)"))
  ;[1 1 1] Collider Overlap
  (`SceneComponent.SetVisibility` (`self.Widget`) true false))

(event `self.Box.OnComponentEndOverlap`
  (params (OverlappedComponent :type "PrimitiveComponent Object Reference") (OtherActor :type "Actor Object Reference") (OtherComp :type "PrimitiveComponent Object Reference") (OtherBodyIndex :type Integer))
  ;[1 1 1] Collider Overlap
  (`SceneComponent.SetVisibility` (`self.Widget`) false false))

(event `self.ShopKeeperMenu`
  (bind _returnvalue (`GameplayStatics.GetPlayerController` 0))
  ;[1 1 1] ShopKeeper Event
  (bind _returnvalue_2 (`|CreateWidget` "/Game/Blueprints/UI/UI_Screens/Extra_Speed.Extra_Speed_C"))
  (`UserWidget.AddToViewport` _returnvalue_2 0)
  (set `PlayerController.bShowMouseCursor` true _returnvalue)
  (`WidgetBlueprintLibrary.SetInputMode_UIOnlyEx` _returnvalue null)
  (`GameplayStatics.SetGamePaused` true))

(fn `UserConstructionScript`)