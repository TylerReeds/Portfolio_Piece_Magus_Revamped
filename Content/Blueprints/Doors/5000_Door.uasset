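; Purchasable door that the player removes by spending 5000 Score.
; Front and back box overlaps each show and hide their own widget, with no check on which actor overlaps.
; The BuyingDoors event, not called within this Blueprint, checks the Player_BP Score, deducts the cost, prints a confirmation and destroys the door.
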(event `self.Box.OnComponentBeginOverlap`
  (params (OverlappedComponent :type "PrimitiveComponent Object Reference") (OtherActor :type "Actor Object Reference") (OtherComp :type "PrimitiveComponent Object Reference") (OtherBodyIndex :type Integer) (bFromSweep :type Boolean) (SweepResult :type "HitResult Structure (by ref)"))
  ;[1 1 1] Overlap for front side
  (`SceneComponent.SetVisibility` (`self.Widget`) true false))

(event `self.Box.OnComponentEndOverlap`
  (params (OverlappedComponent :type "PrimitiveComponent Object Reference") (OtherActor :type "Actor Object Reference") (OtherComp :type "PrimitiveComponent Object Reference") (OtherBodyIndex :type Integer))
  ;[1 1 1] Overlap for front side
  (`SceneComponent.SetVisibility` (`self.Widget`) false false))

(event `self.Box1.OnComponentBeginOverlap`
  (params (OverlappedComponent :type "PrimitiveComponent Object Reference") (OtherActor :type "Actor Object Reference") (OtherComp :type "PrimitiveComponent Object Reference") (OtherBodyIndex :type Integer) (bFromSweep :type Boolean) (SweepResult :type "HitResult Structure (by ref)"))
  ;[1 1 1] Overlap for backside
  (`SceneComponent.SetVisibility` (`self.Widget1`) true false))

(event `self.Box1.OnComponentEndOverlap`
  (params (OverlappedComponent :type "PrimitiveComponent Object Reference") (OtherActor :type "Actor Object Reference") (OtherComp :type "PrimitiveComponent Object Reference") (OtherBodyIndex :type Integer))
  ;[1 1 1] Overlap for backside
  (`SceneComponent.SetVisibility` (`self.Widget1`) false false))

(event `self.BuyingDoors`
  ;[1 1 1] Buying Doors Event
  (bind _asplayer_bp (cast `/Game/Characters/Player_BP` (`GameplayStatics.GetPlayerCharacter` 0)))
  (if (>= (`/Game/Characters/Player_BP.Score` _asplayer_bp) 5000)
    (`KismetSystemLibrary.PrintText` "Door Bought")
    (bind _asplayer_bp_2 (cast `/Game/Characters/Player_BP` (`GameplayStatics.GetPlayerCharacter` 0)))
    (set `/Game/Characters/Player_BP.Score` (- (`/Game/Characters/Player_BP.Score` _asplayer_bp_2) 5000) _asplayer_bp_2)
    (`self.K2_DestroyActor`)))

(fn `UserConstructionScript`)